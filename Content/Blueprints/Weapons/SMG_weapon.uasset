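; SMG weapon Blueprint that sets its ammo, reload and spread stats at construction and copies them into the player's matching primary or secondary slot on equip.
; Fire spends ammo, traces from the camera with random spread, then retraces from the muzzle, though that second result is unused.
; Each shot spawns an impact decal and a tracer; no damage is applied here.
; Reload refills ammo after a delay bracketed by two sounds.
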(event `self.EquipPrimary`
  (bind (_ammocount _maxammo _reloadtime _bulletspread _asfirst_person_character) (`self.SetGunValues`))
  (bind _primaryweapon_name (break `/Game/Blueprints/Gun_data` (`/Game/FirstPersonBP/Blueprints/FirstPersonCharacter.PrimaryWeapon` (cast `/Game/FirstPersonBP/Blueprints/FirstPersonCharacter` (`GameplayStatics.GetPlayerCharacter` 0) :!pure true))))
  (if (`|EnumEquality` _primaryweapon_name "NewEnumerator2")
    (set `/Game/FirstPersonBP/Blueprints/FirstPersonCharacter.PrimaryWeapon` (make `/Game/Blueprints/Gun_data` "NewEnumerator2" "SMG_weapon_C" _ammocount _maxammo _reloadtime _bulletspread) _asfirst_person_character)))

(event `self.EquipSecondary`
  (bind (_ammocount _maxammo _reloadtime _bulletspread _asfirst_person_character) (`self.SetGunValues`))
  (bind _secondaryweapon_name (break `/Game/Blueprints/Gun_data` (`/Game/FirstPersonBP/Blueprints/FirstPersonCharacter.SecondaryWeapon` (cast `/Game/FirstPersonBP/Blueprints/FirstPersonCharacter` (`GameplayStatics.GetPlayerCharacter` 0) :!pure true))))
  (if (`|EnumEquality` _secondaryweapon_name "NewEnumerator2")
    (set `/Game/FirstPersonBP/Blueprints/FirstPersonCharacter.SecondaryWeapon` (make `/Game/Blueprints/Gun_data` "NewEnumerator2" "SMG_weapon_C" _ammocount _maxammo _reloadtime _bulletspread) _asfirst_person_character)))

(event `self.Fire`
  (if (> (`self.AmmoCount`) 0)
    (`self.AmmoCheck`)
    (bind (_muzzle_loc _impactpoint) (`self.LineTrace`))
    (`self.SpawnDecalTracer` _muzzle_loc _impactpoint _impactpoint)))

(event `self.Reload`
  (bind _returnvalue (`self.GetLocationOfPlayer`))
  (`GameplayStatics.PlaySoundAtLocation` "/Game/Files/MilitaryWeapSilver/Sound/Rifle/Wavs/Rifle_Reload01.Rifle_Reload01" _returnvalue (struct) 1.0 1.0 0.0 null null null)
  (`KismetSystemLibrary.Delay` (`self.ReloadTime`))
  (`GameplayStatics.PlaySoundAtLocation` "/Game/Files/MilitaryWeapSilver/Sound/Rifle/Wavs/Rifle_Reload02.Rifle_Reload02" _returnvalue (struct) 1.0 1.0 0.0 null null null)
  (set `self.AmmoCount` (`self.MaxAmmo`)))

(fn `AmmoCheck`
  (`/Engine/EditorBlueprintResources/StandardMacros.DecrementInt` (`self.AmmoCount`)
    (:`  `
      (if (not (`/Game/FirstPersonBP/Blueprints/FirstPersonCharacter.IsReloading` (cast `/Game/FirstPersonBP/Blueprints/FirstPersonCharacter` (`GameplayStatics.GetPlayerCharacter` 0) :!pure true)))
        (`GameplayStatics.PlaySoundAtLocation` "/Game/Files/MilitaryWeapSilver/Sound/Rifle/Wavs/RifleA_Fire02.RifleA_Fire02" (`self.GetLocationOfPlayer`) (struct) 1.0 1.0 0.0 null null null)))))

(fn `LineTrace`
  (returns (`Muzzle Loc` :type "Vector Structure") (ImpactPoint :type "Vector Structure"))
  (bind _bulletspread (`self.BulletSpread`))
  (bind _returnvalue (`SceneComponent.K2_GetComponentLocation` (`self.Muzzle`)))
  (bind _returnvalue_2 (* _bulletspread -1.0))
  (bind _firstpersoncamera (`/Game/FirstPersonBP/Blueprints/FirstPersonCharacter.FirstPersonCamera` (cast `/Game/FirstPersonBP/Blueprints/FirstPersonCharacter` (`GameplayStatics.GetPlayerCharacter` 0) :!pure true)))
  (bind _returnvalue_3 (`SceneComponent.K2_GetComponentLocation` _firstpersoncamera))
  (bind _outhit (`KismetSystemLibrary.LineTraceSingle` _returnvalue_3 (+ (+ (* (`SceneComponent.GetForwardVector` _firstpersoncamera) 20000.0) _returnvalue_3) (`KismetMathLibrary.MakeVector` (`KismetMathLibrary.RandomFloatInRange` _returnvalue_2 _bulletspread) (`KismetMathLibrary.RandomFloatInRange` _returnvalue_2 _bulletspread) (`KismetMathLibrary.RandomFloatInRange` _returnvalue_2 _bulletspread))) "TraceTypeQuery1")) ; Camera Shot
  (bind (_bblockinghit _binitialoverlap _time _distance _location _impactpoint) (`GameplayStatics.BreakHitResult` _outhit))
  (`KismetSystemLibrary.LineTraceSingle` :`Start` _returnvalue :`End` _impactpoint :`TraceChannel` "TraceTypeQuery1" :`TraceColor` (struct :`G` 0.240256 :`B` 1.0 :`A` 1.0)) ; Gun Shot
  (return _returnvalue _impactpoint))

(fn `SpawnDecalTracer`
  (params (Location :type "Vector Structure") (SpawnTransform :type "Vector Structure") (ImpactPoint :type "Vector Structure"))
  (`|SpawnActorFromClass` "/Game/Blueprints/BP_bulletdecal.BP_bulletdecal_C" (`KismetMathLibrary.MakeTransform` SpawnTransform (`KismetMathLibrary.Conv_VectorToRotator` ImpactPoint) (0.025 0.025 0.025)) "Undefined" "OverrideRootScale" null null)
  (if (>= (`KismetMathLibrary.RandomIntegerInRange` 1 10) 0)
    (`|SpawnActorFromClass` "/Game/Blueprints/BP_TracerRounds.BP_TracerRounds_C" (`KismetMathLibrary.MakeTransform` Location (`SceneComponent.K2_GetComponentRotation` (`/Game/FirstPersonBP/Blueprints/FirstPersonCharacter.FirstPersonCamera` (cast `/Game/FirstPersonBP/Blueprints/FirstPersonCharacter` (`GameplayStatics.GetPlayerCharacter` 0) :!pure true))) (0.05 0.05 0.05)) "Undefined" "OverrideRootScale" null null))
  (return))

(fn `UserConstructionScript`
  (`parent.UserConstructionScript`)
  (set `self.MaxAmmo` 16)
  (set `self.AmmoCount` 16)
  (set `self.ReloadTime` 1.0)
  (set `self.BulletSpread` 1000.0)
  (set `self.Name` "NewEnumerator2"))