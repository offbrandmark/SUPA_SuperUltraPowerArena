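; SMG weapon pickup that gives an overlapping FirstPersonCharacter an SMG in a free weapon slot.
; Its Sphere collision stays off briefly after BeginPlay, then turns on as query-only.
; On overlap it tries the primary slot, then the secondary, writing the weapon struct, setting the child actor class and calling that slot's switch function.
; The pickup destroys itself once taken and stays if neither slot qualifies.
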(event `self.ReceiveBeginPlay`
  (`PrimitiveComponent.SetCollisionEnabled` (`self.Sphere`) "NoCollision")
  (`KismetSystemLibrary.Delay` 0.5)
  (`PrimitiveComponent.SetCollisionEnabled` (`self.Sphere`) "QueryOnly"))

(event `self.Sphere.OnComponentBeginOverlap`
  (params (OverlappedComponent :type "PrimitiveComponent Object Reference") (OtherActor :type "Actor Object Reference") (OtherComp :type "PrimitiveComponent Object Reference") (OtherBodyIndex :type Integer) (bFromSweep :type Boolean) (SweepResult :type "HitResult Structure (by ref)"))
  (bind (_asfirst_person_character _bsuccess) (cast `/Game/FirstPersonBP/Blueprints/FirstPersonCharacter` OtherActor :!pure true))
  (bind _primary_weapon_name (break `/Game/Blueprints/Gun_data` (`/Game/FirstPersonBP/Blueprints/FirstPersonCharacter.Primary Weapon` _asfirst_person_character)))
  (bind _secondary_weapon_name (break `/Game/Blueprints/Gun_data` (`/Game/FirstPersonBP/Blueprints/FirstPersonCharacter.Secondary Weapon` _asfirst_person_character)))
  (if _bsuccess
    (if (`|EnumEquality` _primary_weapon_name "NewEnumerator0")
      (set `/Game/FirstPersonBP/Blueprints/FirstPersonCharacter.Primary Weapon` (make `/Game/Blueprints/Gun_data` "NewEnumerator2" "/Game/Blueprints/Weapons/SMG_weapon.SMG_weapon_C" 16 16 1.0 1000.0) _asfirst_person_character)
      (set `/Game/FirstPersonBP/Blueprints/FirstPersonCharacter.WeaponEquipped` 0.0 _asfirst_person_character)
      (`ChildActorComponent.SetChildActorClass` (`.PrimaryWeapon` (`/Game/FirstPersonBP/Blueprints/FirstPersonCharacter.PrimaryWeapon` _asfirst_person_character)) "/Game/Blueprints/Weapons/SMG_weapon.SMG_weapon_C")
      (`/Game/FirstPersonBP/Blueprints/FirstPersonCharacter.PrimaryWeaponSwitch` _asfirst_person_character)
      (`self.K2_DestroyActor`)
      (elif (`|EnumEquality` _secondary_weapon_name "NewEnumerator0")
        (set `/Game/FirstPersonBP/Blueprints/FirstPersonCharacter.Secondary Weapon` (make `/Game/Blueprints/Gun_data` "NewEnumerator2" "/Game/Blueprints/Weapons/SMG_weapon.SMG_weapon_C" 16 16 1.0 1000.0) _asfirst_person_character)
        (set `/Game/FirstPersonBP/Blueprints/FirstPersonCharacter.WeaponEquipped` 0.0 1 _asfirst_person_character)
        (`ChildActorComponent.SetChildActorClass` (`.SecondaryWeapon` (`/Game/FirstPersonBP/Blueprints/FirstPersonCharacter.SecondaryWeapon` _asfirst_person_character)) "/Game/Blueprints/Weapons/SMG_weapon.SMG_weapon_C")
        (`/Game/FirstPersonBP/Blueprints/FirstPersonCharacter.SecondaryWeaponSwitch` _asfirst_person_character)
        (`self.K2_DestroyActor`)))))

(fn `UserConstructionScript`)