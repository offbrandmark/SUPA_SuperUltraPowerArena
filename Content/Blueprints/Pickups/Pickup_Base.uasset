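; Base Blueprint for weapon pickups, declaring empty PickupPrimary and PickupSecondary events.
; On BeginPlay its Sphere's collision is disabled, then set to query-only after a short delay.
; Both overlap handlers are empty.
; Unconnected leftover logic would put a pistol into an empty primary, else secondary, slot, switch to it and destroy the actor, but it never runs.
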(event `self.ReceiveBeginPlay`
  (`PrimitiveComponent.SetCollisionEnabled` (`self.Sphere`) "NoCollision")
  (`KismetSystemLibrary.Delay` 0.5)
  (`PrimitiveComponent.SetCollisionEnabled` (`self.Sphere`) "QueryOnly"))

(event `PickupPrimary`)

(event `PickupSecondary`)

(event `self.StaticMesh.OnComponentBeginOverlap`
  (params (OverlappedComponent :type "PrimitiveComponent Object Reference") (OtherActor :type "Actor Object Reference") (OtherComp :type "PrimitiveComponent Object Reference") (OtherBodyIndex :type Integer) (bFromSweep :type Boolean) (SweepResult :type "HitResult Structure (by ref)")))

(event `self.Sphere.OnComponentEndOverlap`
  (params (OverlappedComponent :type "PrimitiveComponent Object Reference") (OtherActor :type "Actor Object Reference") (OtherComp :type "PrimitiveComponent Object Reference") (OtherBodyIndex :type Integer)))

(fn `UserConstructionScript`)