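; Pistol pickup actor that lets the player equip a pistol in either the primary or secondary weapon slot.
; Its sphere overlap shows a WeaponDisplay widget labeled "Pistol" while the FirstPersonCharacter is in range and removes it on exit.
; PickupPrimary and PickupSecondary events set the matching child actor component on the player character to Pistol_weapon, then destroy the pickup.
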(event `self.Sphere.OnComponentBeginOverlap`
  (params (OverlappedComponent :type "PrimitiveComponent Object Reference") (OtherActor :type "Actor Object Reference") (OtherComp :type "PrimitiveComponent Object Reference") (OtherBodyIndex :type Integer) (bFromSweep :type Boolean) (SweepResult :type "HitResult Structure (by ref)"))
  (if (`.bSuccess` (cast `/Game/FirstPersonBP/Blueprints/FirstPersonCharacter` OtherActor :!pure true))
    (bind _returnvalue (`|CreateWidget` "/Game/FirstPersonBP/Blueprints/WeaponDisplay.WeaponDisplay_C"))
    (set `/Game/FirstPersonBP/Blueprints/WeaponDisplay.Weapon` "Pistol" _returnvalue)
    (`UserWidget.AddToViewport` _returnvalue 0)))

(event `self.Sphere.OnComponentEndOverlap`
  (params (OverlappedComponent :type "PrimitiveComponent Object Reference") (OtherActor :type "Actor Object Reference") (OtherComp :type "PrimitiveComponent Object Reference") (OtherBodyIndex :type Integer))
  (if (`.bSuccess` (cast `/Game/FirstPersonBP/Blueprints/FirstPersonCharacter` OtherActor :!pure true))
    (`Widget.RemoveFromParent` (stale `self.Sphere.OnComponentBeginOverlap` _returnvalue))))

(event `self.ReceiveBeginPlay`
  (`parent.ReceiveBeginPlay`))

(event `self.PickupPrimary`
  (bind _asfirst_person_character (cast `/Game/FirstPersonBP/Blueprints/FirstPersonCharacter` (`GameplayStatics.GetPlayerCharacter` 0)))
  (`ChildActorComponent.SetChildActorClass` (`/Game/FirstPersonBP/Blueprints/FirstPersonCharacter.Primary` _asfirst_person_character) "/Game/Blueprints/Weapons/pistol_weapon.pistol_weapon_C")
  (`self.K2_DestroyActor`))

(event `self.PickupSecondary`
  (bind _asfirst_person_character (cast `/Game/FirstPersonBP/Blueprints/FirstPersonCharacter` (`GameplayStatics.GetPlayerCharacter` 0)))
  (`ChildActorComponent.SetChildActorClass` (`/Game/FirstPersonBP/Blueprints/FirstPersonCharacter.Secondary` _asfirst_person_character) "/Game/Blueprints/Weapons/pistol_weapon.pistol_weapon_C")
  (`self.K2_DestroyActor`))

(fn `UserConstructionScript`
  (`parent.UserConstructionScript`))